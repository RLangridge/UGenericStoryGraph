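; Game mode that serves area-based events and dispatches them as dialogue, decision or combat encounters.
; On BeginPlay it caches the level's single BP_PotentialEventContainer, printing an error otherwise, and uses it to look up events by area name and index.
; ProcessEvent casts the event data asset to its type and passes it to the matching EPRC handler.
; Only the dialogue branch also triggers the UI transition.
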(event `self.ReceiveBeginPlay`
  (bind _outactors (`GameplayStatics.GetAllActorsOfClass` "/Game/Blueprints/Actors/BP_PotentialEventContainer.BP_PotentialEventContainer_C"))
  (if (== (`KismetArrayLibrary.Array_Length` _outactors) 1)
    (set `self.Potential Event Container Reference` (`|GetArrayItem` _outactors))
    (else
      (`KismetSystemLibrary.PrintString` "Error: No event containers in world" true true (struct :`R` 1.0 :`A` 1.0)))))

(event `On Transition UI`
  (params (`UI To Transition` :type "/Game/Blueprints/Interfaces/I_UITransition Interface"))
  (bind _animation_duration (`/Game/Blueprints/Interfaces/I_UITransition.Transition` `UI To Transition`))
  (`KismetSystemLibrary.Delay` _animation_duration))

(fn `Get Event From Area Name`
  (params (`Area Name` :type Name) (`Event Index` :type Integer))
  (returns (`Event Found` :type "/Game/Blueprints/DataAssets/DA_PotentialEvent Object Reference"))
  (return (`|GetArrayItem` (`/Game/Blueprints/Actors/BP_PotentialEventContainer.Get Events From Map` (`self.Potential Event Container Reference`) `Area Name`) `Event Index`)))

(fn `Get Event List`
  (params (`Area Name` :type Name))
  (returns (`Event List` :type "Array of /Game/Blueprints/DataAssets/DA_PotentialEvent Object Reference"))
  (return (`/Game/Blueprints/Actors/BP_PotentialEventContainer.Get Events From Map` (`self.Potential Event Container Reference`) `Area Name`)))

(fn `Process Event`
  (params (`New Event` :type "/Game/Blueprints/DataAssets/DA_PotentialEvent Object Reference") (`UI Reference` :type "/Game/Blueprints/Interfaces/I_UITransition Interface"))
  (bind _asda_dialogue_event (cast `/Game/Blueprints/DataAssets/DA_DialogueEvent` `New Event`)
    (:`then`
      (`self.On Transition UI` `UI Reference`)
      (`/Game/Blueprints/Components/EPRC_Dialogue.On Recieve Initial Data` (`self.EPRC_Dialogue`) _asda_dialogue_event))
    (:`CastFailed`
      (bind _asda_decision_event (cast `/Game/Blueprints/DataAssets/DA_DecisionEvent` `New Event`)
        (:`then`
          (`/Game/Blueprints/Components/EPRC_Decision.On Receive Initial Data` (`self.EPRC_Decision`) _asda_decision_event))
        (:`CastFailed`
          (bind _asda_combat_event (cast `/Game/Blueprints/DataAssets/DA_CombatEvent` `New Event`))
          (`/Game/Blueprints/Components/EPRC_Combat.On Receive Initial Data` (`self.EPRC_Combat`) _asda_combat_event))))))

(fn `UserConstructionScript`)