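; Dialogue component that plays a sequence of dialogue lines from a supplied DialogueData asset or struct through a UI_DialogueProcessor widget.
; Receiving data creates the widget if needed, adds it to the viewport, passes it the background and a self reference, then shows the first line.
; An iterator steps through speaker name, icon, avatar and text on each NextDialogue call, printing a debug message at the end.
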(event `On Recieve Initial Data`
  (params (`Dialogue Data` :type "/Game/Blueprints/DataAssets/DA_DialogueEvent Object Reference"))
  (set `self.Dialogue Data` `Dialogue Data`)
  (`self.Setup UI`)
  (`/Game/Blueprints/UI/UI_DialogueProcessor.Initial Setup` (`self.Dialogue Processor Widget Ref`) (`/Game/Blueprints/DataAssets/DA_DialogueEvent.Background Image` (`self.Dialogue Data`)) self)
  (`self.Set Dialogue`))

(event `Next Dialogue`
  (if (`self.Are We At The End Of Dialogue?`)
    (`KismetSystemLibrary.PrintString` "Finished Dialogue")
    (else
      (`self.Set Dialogue`))))

(fn `Are We At The End Of Dialogue?`
  (returns (Yes :type Boolean))
  (return (== (`self.Iterator`) (`KismetArrayLibrary.Array_Length` (`/Game/Blueprints/DataAssets/DA_DialogueEvent.Dialogue` (`self.Dialogue Data`))))))

(fn `Set Dialogue`
  (bind (_speakericon _speakeravatar _dialogue _nameofspeaker) (break `/Game/Blueprints/Structs/STR_DialogueData` (`|GetArrayItem` (`/Game/Blueprints/DataAssets/DA_DialogueEvent.Dialogue` (`self.Dialogue Data`)) (`self.Iterator`))))
  (`/Game/Blueprints/UI/UI_DialogueProcessor.Receive Dialogue` (`self.Dialogue Processor Widget Ref`) _speakericon _speakeravatar _dialogue _nameofspeaker)
  (`/Engine/EditorBlueprintResources/StandardMacros.IncrementInt` (`self.Iterator`)))

(fn `Setup UI`
  (bind _dialogue_processor_widget_ref (`self.Dialogue Processor Widget Ref`))
  (`/Engine/EditorBlueprintResources/StandardMacros.IsValid` _dialogue_processor_widget_ref
    (:`Is Valid`
      _)
    (:`Is Not Valid`
      (bind _returnvalue (`|CreateWidget` "/Game/Blueprints/UI/UI_DialogueProcessor.UI_DialogueProcessor_C"))
      (set `self.Dialogue Processor Widget Ref` _returnvalue)))
  (`UserWidget.AddToViewport` _dialogue_processor_widget_ref 0))